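; Multiplayer projectile actor that flies forward, damages pawns and expires after a set lifetime.
; The server moves it each tick without sweep and handles sphere overlaps, ignoring its owner and other projectiles.
; A BP_MultiplayerPawn hit applies damage and multicasts an explosion effect, while other hits destroy it without the effect.
; Both impacts and the lifetime timer end through a server event that destroys the actor.
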(event `self.ReceiveBeginPlay`
  ;[1 1 1] EndOfLife
  (`KismetSystemLibrary.K2_SetTimerDelegate` (delegate `EndOfLife`) (`self.TTL`)))

(event `EndOfLife`
  ;[1 1 1] EndOfLife
  (`self.server_end_of_life`))

(event `server_end_of_life`
  ;[1 1 1] EndOfLife
  (`self.K2_DestroyActor`))

(event `server_move`
  (params (DeltaTime :type "Float (double-precision)"))
  ;[1 1 1] Projectile moving
  (`self.K2_SetActorLocation` (+ (`self.K2_GetActorLocation`) (* (`self.GetActorForwardVector`) (* DeltaTime (`self.Speed`))))))

(event `self.ReceiveTick`
  (params (DeltaSeconds :type "Float (single-precision)"))
  ;[1 1 1] Projectile moving
  (if (`KismetSystemLibrary.IsServer`)
    (`self.server_move` DeltaSeconds)))

(event `self.Sphere1.OnComponentBeginOverlap`
  (params (OverlappedComponent :type "PrimitiveComponent Object Reference") (OtherActor :type "Actor Object Reference") (OtherComp :type "PrimitiveComponent Object Reference") (OtherBodyIndex :type Integer) (bFromSweep :type Boolean) (SweepResult :type "HitResult Structure (by ref)"))
  ;[1 1 1] Collision
  (if (`KismetSystemLibrary.IsServer`)
    (`self.server_collision` OtherActor (`self.K2_GetActorLocation`))))

(event `server_collision`
  (params (`Other Actor` :type "Actor Object Reference") (Location :type "Vector Structure"))
  ;[1 1 1] Collision
  (if (!= `Other Actor` (`self.GetOwner`))
    (bind _asbp_multiplayer_pawn (cast `/Game/MyContent/BP/BP_MultiplayerPawn` `Other Actor`)
      (:`then`
        (`/Game/MyContent/BP/BP_MultiplayerPawn.TakeDamage` _asbp_multiplayer_pawn (`self.Damage`))
        (`self.MulticastSpawnHitEffect` Location))
      (:`CastFailed`
        (cast `/Game/MyContent/BP/BP_Projectile` `Other Actor`
          (:`CastFailed`
            _))))
    (`self.EndOfLife`)))

(event `SpawnHitEffect`
  (params (`Hit Location` :type "Vector Structure"))
  (`GameplayStatics.SpawnEmitterAtLocation` "/Game/StarterContent/Particles/P_Explosion.P_Explosion" `Hit Location`))

(event `MulticastSpawnHitEffect`
  (params (Location :type "Vector Structure"))
  (`self.SpawnHitEffect` Location))

(fn `UserConstructionScript`)