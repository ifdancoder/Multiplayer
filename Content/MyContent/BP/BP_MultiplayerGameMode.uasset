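; Multiplayer game mode that assigns players to two teams and rebalances them when someone leaves.
; On PostLogin, it puts each BP_MultiplayerPlayerController on the smaller team, favoring Team 1 on ties, and sets its team ID.
; Logout removes the controller, then shifts a team's first player: Team 1 to 2 if Team 2's lead is under two, reverse if over two.
; The moved controller gets its new ID and a Rebalancing call.
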(event `self.K2_PostLogin`
  (params (NewPlayer :type "PlayerController Object Reference"))
  (bind _asbp_multiplayer_player_controller (cast `/Game/MyContent/BP/BP_MultiplayerPlayerController` NewPlayer)
    (:`then`
      (if (< (`KismetArrayLibrary.Array_Length` (`self.Team2Controllers`)) (`KismetArrayLibrary.Array_Length` (`self.Team1Controllers`)))
        (`/Game/MyContent/BP/BP_MultiplayerPlayerController.SetTeamID` _asbp_multiplayer_player_controller 2)
        (`KismetArrayLibrary.Array_Add` (`self.Team2Controllers`) _asbp_multiplayer_player_controller)
        (else
          (`/Game/MyContent/BP/BP_MultiplayerPlayerController.SetTeamID` _asbp_multiplayer_player_controller 1)
          (`KismetArrayLibrary.Array_Add` (`self.Team1Controllers`) _asbp_multiplayer_player_controller))))
    (:`CastFailed`
      (`KismetSystemLibrary.PrintString` "PostLogin error :("))))

(event `self.K2_OnLogout`
  (params (ExitingController :type "Controller Object Reference"))
  (bind _team2controllers (`self.Team2Controllers`))
  (bind _team1controllers (`self.Team1Controllers`))
  (bind _asbp_multiplayer_player_controller (cast `/Game/MyContent/BP/BP_MultiplayerPlayerController` ExitingController))
  (bind _returnvalue (`KismetArrayLibrary.Array_Find` _team2controllers _asbp_multiplayer_player_controller))
  (if (== _returnvalue -1)
    (bind _returnvalue_2 (`KismetArrayLibrary.Array_Find` _team1controllers _asbp_multiplayer_player_controller))
    (if (not (== _returnvalue_2 -1))
      (`KismetArrayLibrary.Array_Remove` _team1controllers _returnvalue_2))
    (else
      (`KismetArrayLibrary.Array_Remove` _team2controllers _returnvalue)))
  (`self.Rebalancing teams`))

(event `Rebalancing teams`
  (bind _team1controllers (`self.Team1Controllers`))
  (bind _team2controllers (`self.Team2Controllers`))
  (bind _movingplayer (`self.MovingPlayer`))
  (bind _returnvalue (- (`KismetArrayLibrary.Array_Length` (`self.Team2Controllers`)) (`KismetArrayLibrary.Array_Length` (`self.Team1Controllers`))))
  (if (< _returnvalue 2)
    (set `self.MovingPlayer` (`|GetArrayItem` _team1controllers))
    (`KismetArrayLibrary.Array_Remove` _team1controllers)
    (`KismetArrayLibrary.Array_Add` _team2controllers _movingplayer)
    (`/Game/MyContent/BP/BP_MultiplayerPlayerController.SetTeamID` _movingplayer 2)
    (`/Game/MyContent/BP/BP_MultiplayerPlayerController.Rebalancing` _movingplayer :!label _label)
    (elif (> _returnvalue 2)
      (set `self.MovingPlayer` (`|GetArrayItem` _team2controllers))
      (`KismetArrayLibrary.Array_Remove` _team2controllers)
      (`KismetArrayLibrary.Array_Add` _team1controllers _movingplayer)
      (`/Game/MyContent/BP/BP_MultiplayerPlayerController.SetTeamID` _movingplayer 1)
      (goto _label))))

(fn `UserConstructionScript`)