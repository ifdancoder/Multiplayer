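; Multiplayer game instance that hosts and searches for LAN sessions.
; CreateGame creates a 16-slot LAN session, then opens Lvl1 as a listen server.
; GetGames searches for sessions and only prints each result's server name, player counts and ping, with no join logic.
; Session failures and network or travel errors are reported through on-screen debug prints.
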(event `Create Game`
  (`CreateSessionCallbackProxy.CreateSession` (`GameplayStatics.GetPlayerController` 0) 16 true
    (:`OnSuccess`
      (`GameplayStatics.OpenLevel` "Lvl1" true "listen"))
    (:`OnFailure`
      (`KismetSystemLibrary.PrintString` "Error with creating lobby :("))))

(event `GetGames`
  (bind _results (`FindSessionsCallbackProxy.FindSessions` (`GameplayStatics.GetPlayerController` 0) 20 true)
    (:`OnSuccess`
      (for _array_element _results
        (`KismetSystemLibrary.PrintString` (`KismetStringLibrary.Concat_StrStr` "Server:" (`FindSessionsCallbackProxy.GetServerName` _array_element) "Players:" (`KismetStringLibrary.Conv_IntToString` (`FindSessionsCallbackProxy.GetCurrentPlayers` _array_element)) "/" (`KismetStringLibrary.Conv_IntToString` (`FindSessionsCallbackProxy.GetMaxPlayers` _array_element)) "Ping:" (`KismetStringLibrary.Conv_IntToString` (`FindSessionsCallbackProxy.GetPingInMs` _array_element))))))
    (:`OnFailure`
      (`KismetSystemLibrary.PrintString` "Error with finding games :("))))

(event `self.HandleNetworkError`
  (params (FailureType :type "ENetworkFailure Enum" :default "NetDriverAlreadyExists") (bIsServer :type Boolean))
  (`KismetSystemLibrary.PrintString` (`KismetStringLibrary.Concat_StrStr` "Network error:" (`|GetEnumeratorNameAsString` FailureType) "on server?" (`KismetStringLibrary.Conv_BoolToString` bIsServer))))

(event `self.HandleTravelError`
  (params (FailureType :type "ETravelFailure Enum" :default "NoLevel"))
  (`KismetSystemLibrary.PrintString` (`|GetEnumeratorNameAsString` FailureType)))