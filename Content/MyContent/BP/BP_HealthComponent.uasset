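; BP_HealthComponent is an actor component that tracks health and max health for its owner in multiplayer.
; A server event sets both values, and TakeDamage subtracts from Health.
; The Health RepNotify pushes the percentage to a BP_MultiplayerPawn owner's HP bar, or destroys the owner when health reaches zero or below.
; Helper functions return the health fraction and whether the values are initialized.
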(event `server_set_hp`
  (params (`Max HP` :type "Float (double-precision)"))
  (bind _output_get (set `self.MaxHealth` `Max HP`))
  (set `self.Health` _output_get))

(fn `Get Percent`
  (returns (Percent :type "Float (double-precision)"))
  (return (/ (`self.Health`) (`self.MaxHealth`))))

(fn `is Valid`
  (returns (Validness :type Boolean))
  (return (and (!= (`self.MaxHealth`) 0.0) (!= (`self.Health`) -1.0))))

(fn `OnRep_Health`
  (bind _health (`self.Health`))
  (if (> _health 0.0)
    (bind _asbp_multiplayer_pawn (cast `/Game/MyContent/BP/BP_MultiplayerPawn` (`self.GetOwner`)))
    (`/Game/MyContent/BP/BP_MultiplayerPawn.SetPercentHPBar` _asbp_multiplayer_pawn (/ _health (`self.MaxHealth`)))
    (else
      (`Actor.K2_DestroyActor` (`self.GetOwner`)))))

(fn `TakeDamage`
  (params (Damage :type "Float (double-precision)"))
  (set `self.Health` (- (`self.Health`) Damage)))